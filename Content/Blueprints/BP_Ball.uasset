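; BP_Ball is a physics-driven ball that is launched from the player's paddle and plays sounds on impact.
; FireBall applies a fixed velocity-change impulse to the Ball component and sets IsFired on the controlled BP_Paddle.
; Hit events cast the other actor to choose a money-collect sound or a bleep, staying silent for boundaries and while the paddle's KeyHeld is true.
; A horizontal speed clamp is present but disconnected.
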(event `self.ReceiveBeginPlay`)

(event `self.ReceiveTick`
  (params (DeltaSeconds :type "Float (single-precision)"))
  ;[1 1 1] Limit the max velocity (Not Working)
)

(event `self.Ball.OnComponentHit`
  (params (HitComponent :type "PrimitiveComponent Object Reference") (OtherActor :type "Actor Object Reference") (OtherComp :type "PrimitiveComponent Object Reference") (NormalImpulse :type "Vector Structure") (Hit :type "HitResult Structure (by ref)"))
  (cast `/Game/Blueprints/BP_Money` OtherActor
    (:`then`
      ;[1 1 1] Limit the max velocity (Not Working)
      (`GameplayStatics.PlaySound2D` "/Game/Sound/393777__pogmog__money-collect-1.393777__pogmog__money-collect-1" 0.5))
    (:`CastFailed`
      (cast `/Game/Blueprints/BP_Boundary` OtherActor
        (:`CastFailed`
          (bind _asbp_paddle (cast `/Game/Blueprints/BP_Paddle` OtherActor)
            (:`then`
              (if (not (`/Game/Blueprints/BP_Paddle.keyHeld` _asbp_paddle))
                (`GameplayStatics.PlaySound2D` "/Game/Sound/86101__scarkord__pss-bleep.86101__scarkord__pss-bleep" 0.5 :!label _label)))
            (:`CastFailed`
              (goto _label))))))))

(fn `FireBall`
  (`PrimitiveComponent.AddImpulse` (`self.Ball`) (500.0 -500.0 0.0) "None" true)
  (bind _asbp_paddle (cast `/Game/Blueprints/BP_Paddle` (`Controller.K2_GetPawn` (`GameplayStatics.GetPlayerController` 0))))
  (set `/Game/Blueprints/BP_Paddle.isFired` true _asbp_paddle))

(fn `UserConstructionScript`)