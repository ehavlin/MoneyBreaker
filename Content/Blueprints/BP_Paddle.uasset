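; BP_Paddle is the player-controlled paddle that moves left and right by physics impulse and holds, launches and catches the ball.
; It spawns BP_Ball at its Arrow on BeginPlay, pinning it there each tick until Fire launches it.
; Holding Grab when the ball hits the paddle re-attaches it by clearing IsFired and velocity.
; Reset also recalls the ball and calls CheckLives on BP_Boundary; Pause opens UI_Pause.
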(event `self.ReceiveBeginPlay`
  (`self.SpawnBall`))

(event `InputAxis|Left/Right`
  (params (AxisValue :type "Float (single-precision)"))
  ;[1 1 1] Movement
  (`PrimitiveComponent.AddImpulse` (`self.Paddle`) (`KismetMathLibrary.MakeVector` (* AxisValue 8000.0)) "None" false))

(event `InputAction|Fire`
  (params (Key :type "Key Structure"))
  ;[1 1 1] Launch the ball when input is given
  (:`Pressed`
    (if (not (`self.isFired`))
      (`/Game/Blueprints/BP_Ball.FireBall` (`self.Ball`)))))

(event `self.ReceiveTick`
  (params (DeltaSeconds :type "Float (single-precision)"))
  ;[1 1 1] Change ball location to paddle's location only if it has not been fired
  (if (not (`self.isFired`))
    (`self.K2_SetActorLocation` (`self.Ball`) (`SceneComponent.K2_GetComponentLocation` (`self.Arrow`)) false false)))

(event `InputAction|Grab`
  (params (Key :type "Key Structure"))
  ;[1 1 1] Check to see if the grab button is being held
  (:`Pressed`
    (set `self.keyHeld` true))
  (:`Released`
    (set `self.keyHeld` false)))

(event `InputAction|ResetBall`
  (params (Key :type "Key Structure"))
  (:`Pressed`
    (set `self.isFired` false)
    (`PrimitiveComponent.SetPhysicsLinearVelocity` (`/Game/Blueprints/BP_Ball.Ball` (`self.Ball`)) (0.0 0.0 0.0) false "None")
    (bind _outactors (`GameplayStatics.GetAllActorsOfClass` "/Game/Blueprints/BP_Boundary.BP_Boundary_C"))
    (`/Game/Blueprints/BP_Boundary.checkLives` _outactors)))

(event `InputAction|Pause`
  (params (Key :type "Key Structure"))
  (bind _returnvalue (`GameplayStatics.GetPlayerController` 0))
  ;[1 1 1] Pause game when P is pressed
  (:`Pressed`
    (bind _returnvalue_2 (`|CreateWidget` "/Game/UI/UI_Pause.UI_Pause_C"))
    (`UserWidget.AddToViewport` _returnvalue_2 0)
    (set `PlayerController.bShowMouseCursor` true _returnvalue)
    (`WidgetBlueprintLibrary.SetInputMode_UIOnlyEx` _returnvalue)
    (`GameplayStatics.SetGamePaused` true)))

(event `self.Paddle.OnComponentHit`
  (params (HitComponent :type "PrimitiveComponent Object Reference") (OtherActor :type "Actor Object Reference") (OtherComp :type "PrimitiveComponent Object Reference") (NormalImpulse :type "Vector Structure") (Hit :type "HitResult Structure (by ref)"))
  ;[1 1 1] Grab the ball if X is held
  (bind _asbp_ball (cast `/Game/Blueprints/BP_Ball` OtherActor))
  (if (`self.keyHeld`)
    (set `self.isFired` false)
    (`PrimitiveComponent.SetPhysicsLinearVelocity` (`/Game/Blueprints/BP_Ball.Ball` _asbp_ball) (0.0 0.0 0.0) false "None")))

(fn `SpawnBall`
  (bind _returnvalue (`|SpawnActorFromClass` "/Game/Blueprints/BP_Ball.BP_Ball_C" (`KismetMathLibrary.MakeTransform` (`SceneComponent.K2_GetComponentLocation` (`self.Arrow`)) (struct) (0.25 0.25 0.25)) "Undefined" "OverrideRootScale" null null))
  (set `self.Ball` _returnvalue))

(fn `UserConstructionScript`)