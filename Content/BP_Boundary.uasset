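; BP_Boundary is the kill zone that destroys a BP_Ball hitting its cube and costs the player a life.
; On hit, CheckLives decrements Lives in BP_GameMode and, when none remain, shows UI_Lose, switches to UI-only input and pauses the game.
; The hit event then has the controlled BP_Paddle spawn a new ball and clears IsFired, without checking whether the game was lost.
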(event `self.Cube.OnComponentHit`
  (params (HitComponent :type "PrimitiveComponent Object Reference") (OtherActor :type "Actor Object Reference") (OtherComp :type "PrimitiveComponent Object Reference") (NormalImpulse :type "Vector Structure") (Hit :type "HitResult Structure (by ref)"))
  ;[1 1 1] Destroy ball on impact and check lose condition. If the the player still has lives, spawn a new ball
  (bind _asbp_ball (cast `/Game/BP_Ball` OtherActor))
  (`self.K2_DestroyActor` _asbp_ball)
  (`self.checkLives`)
  (bind _asbp_paddle (cast `/Game/BP_Paddle` (`Controller.K2_GetPawn` (`GameplayStatics.GetPlayerController` 0))))
  (`/Game/BP_Paddle.SpawnBall` _asbp_paddle)
  (set `/Game/BP_Paddle.isFired` false _asbp_paddle))

(fn `checkLives`
  (bind _returnvalue (`GameplayStatics.GetPlayerController` 0))
  (bind _asbp_game_mode (cast `/Game/BP_GameMode` (`GameplayStatics.GetGameMode`)))
  (bind _result (`/Engine/EditorBlueprintResources/StandardMacros.DecrementInt` (`/Game/BP_GameMode.Lives` _asbp_game_mode))
    (:`  `
      (if (not (> _result 0))
        (bind _returnvalue_2 (`|CreateWidget` "/Game/UI_Lose.UI_Lose_C"))
        (`UserWidget.AddToViewport` _returnvalue_2 0)
        (set `PlayerController.bShowMouseCursor` true _returnvalue)
        (`WidgetBlueprintLibrary.SetInputMode_UIOnlyEx` _returnvalue)
        (`GameplayStatics.SetGamePaused` true)))))

(fn `UserConstructionScript`)