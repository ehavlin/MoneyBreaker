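; BP_Money is a collectible money pickup that the ball destroys on impact to earn score.
; When its MoneyWad component is hit by BP_Ball, it destroys itself, adds a fixed amount to the BP_GameMode score and runs CheckWinCondition.
; That function counts remaining BP_Money actors and, when none are left, shows the UI_Win widget, enables the cursor with UI-only input and pauses the game.
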(event `self.MoneyWad.OnComponentHit`
  (params (HitComponent :type "PrimitiveComponent Object Reference") (OtherActor :type "Actor Object Reference") (OtherComp :type "PrimitiveComponent Object Reference") (NormalImpulse :type "Vector Structure") (Hit :type "HitResult Structure (by ref)"))
  ;[1 1 1] Destroys Money actor on impact with the ball and then checks for win condition
  (cast `/Game/BP_Ball` OtherActor)
  (`self.K2_DestroyActor`)
  (bind _asbp_game_mode (cast `/Game/BP_GameMode` (`GameplayStatics.GetGameMode`)))
  (set `/Game/BP_GameMode.Score` (+ (`/Game/BP_GameMode.Score` _asbp_game_mode) 50000) _asbp_game_mode)
  (`self.CheckWinCondition`))

(fn `CheckWinCondition`
  (bind _returnvalue (`GameplayStatics.GetPlayerController` 0))
  (bind _outactors (`GameplayStatics.GetAllActorsOfClass` "BP_Money_C"))
  (if (== (`KismetArrayLibrary.Array_Length` _outactors) 0)
    (bind _returnvalue_2 (`|CreateWidget` "/Game/UI_Win.UI_Win_C"))
    (`UserWidget.AddToViewport` _returnvalue_2 0)
    (set `PlayerController.bShowMouseCursor` true _returnvalue)
    (`WidgetBlueprintLibrary.SetInputMode_UIOnlyEx` _returnvalue)
    (`GameplayStatics.SetGamePaused` true)))

(fn `UserConstructionScript`)