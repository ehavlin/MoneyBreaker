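; BP_Ball is a physics-driven ball that works with the player's BP_Paddle.
; FireBall launches it with a fixed diagonal velocity-change impulse, then sets IsFired on the BP_Paddle controlled by player 0.
; A clamp on horizontal speed that preserves vertical velocity is left unconnected to Tick and marked as not working, so it never runs.
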(event `self.ReceiveBeginPlay`)

(event `self.ReceiveTick`
  (params (DeltaSeconds :type "Float (single-precision)"))
  ;[1 1 1] Limit the max velocity (Not Working)
)

(fn `FireBall`
  (`PrimitiveComponent.AddImpulse` (`self.Ball`) (500.0 -500.0 0.0) "None" true)
  (bind _asbp_paddle (cast `/Game/BP_Paddle` (`Controller.K2_GetPawn` (`GameplayStatics.GetPlayerController` 0))))
  (set `/Game/BP_Paddle.isFired` true _asbp_paddle))

(fn `UserConstructionScript`)